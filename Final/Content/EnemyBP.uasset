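; EnemyBP is an enemy actor that kills the hero on contact and can itself be destroyed by damage.
; It sets its HP on BeginPlay, and a DecreaseHP event subtracts a given amount, destroying the actor once HP runs out.
; A CollisionBox overlap casts the other actor to HeroBP and calls Die on it.
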(event `self.ReceiveBeginPlay`
  (set `self.HP` 100.0))

(event `/Game/DamaeInterface.DecreaseHP`
  (params (amount :type "Float (single-precision)"))
  (bind _output_get (set `self.HP` (- (`self.HP`) amount)))
  (if (<= _output_get 0.0)
    (`self.K2_DestroyActor`)))

(event `self.CollisionBox.OnComponentBeginOverlap`
  (params (OverlappedComponent :type "PrimitiveComponent Object Reference") (OtherActor :type "Actor Object Reference") (OtherComp :type "PrimitiveComponent Object Reference") (OtherBodyIndex :type Integer) (bFromSweep :type Boolean) (SweepResult :type "HitResult Structure (by ref)"))
  (bind _ashero_bp (cast `/Game/HeroBP` OtherActor))
  (`/Game/HeroBP.Die` _ashero_bp))

(fn `UserConstructionScript`)