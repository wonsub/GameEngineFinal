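; GunBP is a gun actor that serves as a pickup for HeroBP and can fire bullets.
; When an unequipped hero overlaps its Sphere, it sets IsEquipped, calls the hero's Equip, prints a message and destroys itself.
; StartFiring fires immediately and sets a timer on Fire by function name, which StopFiring clears.
; Each Fire spawns a Bullet at the FirePoint transform.
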(event `self.Sphere.OnComponentBeginOverlap`
  (params (OverlappedComponent :type "PrimitiveComponent Object Reference") (OtherActor :type "Actor Object Reference") (OtherComp :type "PrimitiveComponent Object Reference") (OtherBodyIndex :type Integer) (bFromSweep :type Boolean) (SweepResult :type "HitResult Structure (by ref)"))
  (bind _ashero_bp (cast `/Game/HeroBP` OtherActor))
  (if (not (`/Game/HeroBP.isEquipped` _ashero_bp))
    (set `/Game/HeroBP.isEquipped` true _ashero_bp)
    (`/Game/HeroBP.Equip` _ashero_bp)
    (`KismetSystemLibrary.PrintString` "Equipped")
    (`self.K2_DestroyActor`)))

(event `Fire`
  (`|SpawnActorFromClass` "/Game/Bullet.Bullet_C" (`SceneComponent.K2_GetComponentToWorld` (`self.FirePoint`)) "Undefined" "OverrideRootScale"))

(event `StopFiring`
  (`KismetSystemLibrary.K2_ClearTimer` null "Fire"))

(event `StartFiring`
  (`self.Fire`)
  (`KismetSystemLibrary.K2_SetTimer` null "Fire"))

(fn `UserConstructionScript`)