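; Player hero Blueprint for what appears to be a cursor-aimed shooter, with world-axis movement and rotation derived from the movement input.
; BeginPlay spawns a MousePointBP marker and shows the cursor; left click moves the marker to the cursor hit and fires while IsEquipped, stopping on release.
; Equip spawns a GunBP on the mesh's GunSocket.
; Die disables input and movement, then restarts the level after a delay.
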(event `self.ReceiveBeginPlay`
  (bind _returnvalue (`|SpawnActorFromClass` "/Game/UI/MousePointBP.MousePointBP_C" (`KismetMathLibrary.Conv_VectorToTransform` (`self.K2_GetActorLocation`)) "Undefined" "OverrideRootScale"))
  (set `self.MouseClickPoint` _returnvalue)
  (set `PlayerController.bShowMouseCursor` true (`GameplayStatics.GetPlayerController` 0)))

(event `InputAction|LeftMouseClicked`
  (params (Key :type "Key Structure" :default "AnyKey"))
  (bind _gun (`self.Gun`))
  (bind _isequipped (`self.isEquipped`))
  (:`Pressed`
    (`self.K2_SetActorLocation` (`self.MouseClickPoint`) (`.Location` (`GameplayStatics.BreakHitResult` (`PlayerController.GetHitResultUnderCursorByChannel` (`GameplayStatics.GetPlayerController` 0) "TraceTypeQuery1" true))) false false)
    (if _isequipped
      (`/Game/GunBP.StartFiring` _gun)))
  (:`Released`
    (if _isequipped
      (`/Game/GunBP.StopFiring` _gun))))

(event `InputAxis|MoveForwardBackward`
  (params (AxisValue :type "Float (single-precision)"))
  (`self.AddMovementInput` (1.0 0.0 0.0) AxisValue)
  (if true :!label _label
    (`self.K2_SetActorRotation` (`KismetMathLibrary.Conv_VectorToRotator` (`KismetMathLibrary.MakeVector` AxisValue (stale `InputAxis|MoveLeftRight` AxisValue))))))

(event `InputAxis|MoveLeftRight`
  (params (AxisValue :type "Float (single-precision)"))
  (`self.AddMovementInput` (0.0 1.0 0.0) AxisValue)
  (goto _label))

(event `Die`
  (`self.DisableInput` (`GameplayStatics.GetPlayerController` 0))
  (`CharacterMovementComponent.DisableMovement` (`self.CharacterMovement`))
  (`KismetSystemLibrary.PrintString` "You Die")
  (`KismetSystemLibrary.Delay` 2.0)
  (`KismetSystemLibrary.ExecuteConsoleCommand` "RestartLevel"))

(event `Equip`
  (bind _returnvalue (`|SpawnActorFromClass` "/Game/GunBP.GunBP_C" (`SceneComponent.K2_GetComponentToWorld` (`self.Mesh`)) "Undefined" "OverrideRootScale"))
  (bind _output_get (set `self.Gun` _returnvalue))
  (`self.K2_AttachToComponent` _output_get (`self.Mesh`) "GunSocket" "SnapToTarget" "SnapToTarget" "KeepWorld" true))

(fn `UserConstructionScript`)